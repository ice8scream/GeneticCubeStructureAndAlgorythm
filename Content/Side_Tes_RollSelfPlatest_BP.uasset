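; Functional test Blueprint that checks a Side's plate rolling in both directions.
; It resets the plates to Default, rolls them one way and compares them to the expected RightRoll array, then rolls back and expects Default again.
; On a mismatch it fails with a message listing the actual and expected plate enums; otherwise it reports success.
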(event `self.ReceivePrepareTest`
  (set `/Game/Side_BP.Plates` (`self.Default`) (`self.Side`)))

(event `self.ReceiveStartTest`
  (bind _side (`self.Side`))
  (`/Game/Side_BP.RollSelfPlates` (`self.Side`) false)
  (bind _plates (`/Game/Side_BP.GetPlates` (`self.Side`)))
  (set `self.Check` _plates)
  (set `self.Controll` (`self.RightRoll`))
  (if (`KismetArrayLibrary.Array_Identical` (`self.Check`) (`self.RightRoll`))
    (`/Game/Side_BP.RollSelfPlates` _side true)
    (bind _plates_2 (`/Game/Side_BP.GetPlates` _side))
    (set `self.Check` _plates_2)
    (set `self.Controll` (`self.Default`))
    (if (`KismetArrayLibrary.Array_Identical` (`self.Check`) (`self.Default`))
      (`self.FinishTest` "Succeeded" "Clocwice and Counter Clocwise rotation succeeded")
      (else
        (for _array_element (`self.Check`) :!label _label
          (set `self.ErrMessage` (`KismetStringLibrary.Concat_StrStr` (`self.ErrMessage`) " " (`|GetEnumeratorNameAsString` _array_element))))
        (set `self.ErrMessage` (`KismetStringLibrary.Concat_StrStr` (`self.ErrMessage`) " !="))
        (for _array_element_2 (`self.Controll`)
          (set `self.ErrMessage` (`KismetStringLibrary.Concat_StrStr` (`self.ErrMessage`) " " (`|GetEnumeratorNameAsString` _array_element_2))))
        (`self.FinishTest` "Failed" (`self.ErrMessage`))))
    (else
      (goto _label))))

(fn `UserConstructionScript`)